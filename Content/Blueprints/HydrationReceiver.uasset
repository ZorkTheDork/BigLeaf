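; HydrationReceiver tracks how much hydration its owner receives from the hydration zones registered with it.
; Zones are added to and removed from a set, and each change re-sums their strengths, capped at 255, then signals that the resource changed.
; On BeginPlay it clears the set and binds to the Fox game mode's refresh event so the level can also be recomputed on demand.
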(event `self.ReceiveBeginPlay`
  (bind _asfox_game_mode (`/Game/Blueprints/ActorComponentMacros.GetFoxGameMode`))
  (add `/Game/Blueprints/GameMode/BigLeafGameMode.RefreshResourceReceivers` _asfox_game_mode (delegate `Event RefreshResourceRecieivers`))
  (`BlueprintSetLibrary.Set_Clear` (`self.HydrationZones`)))

(event `Event RefreshResourceRecieivers`
  (`self.RefreshHydrationLevelReceiving`))

(fn `AddHydrationZone`
  (params (HydrationZone :type "/Game/Blueprints/HydrationZone Object Reference"))
  (`BlueprintSetLibrary.Set_Add` (`self.HydrationZones`) HydrationZone)
  (`self.RefreshHydrationLevelReceiving`))

(fn `GetCurrentHydrationLevel`
  (returns (HydrationLevel :type Integer))
  (return (`self.HydrationLevelReceiving`)))

(fn `PrintElements`
  (params (SetOfThings :type "Set of /Game/Blueprints/HydrationZone Object Reference"))
  (bind _result (`BlueprintSetLibrary.Set_ToArray` SetOfThings))
  (for _array_element _result
    (`KismetSystemLibrary.PrintString` (`KismetSystemLibrary.GetDisplayName` _array_element))))

(fn `RefreshHydrationLevelReceiving`
  (locals (totalEnergyOfZones :type Integer))
  (bind _totalenergyofzones (`local.totalEnergyOfZones`))
  (set `local.totalEnergyOfZones` 0)
  (bind _result (`BlueprintSetLibrary.Set_ToArray` (`self.HydrationZones`)))
  (for _array_element _result
    (set `local.totalEnergyOfZones` (`KismetMathLibrary.Min` (+ (`/Game/Blueprints/HydrationZone.HydrationStrength` _array_element) _totalenergyofzones) 255)))
  (set `self.HydrationLevelReceiving` _totalenergyofzones)
  (`self.ResourceChanged`)
  (return))

(fn `RemoveHydrationZone`
  (params (HydrationZone :type "/Game/Blueprints/HydrationZone Object Reference"))
  (`BlueprintSetLibrary.Set_Remove` (`self.HydrationZones`) HydrationZone)
  (`self.RefreshHydrationLevelReceiving`))