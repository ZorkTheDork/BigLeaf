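; TimeOfDaySolarEnergyZone is a solar energy zone whose strength follows the time of day through the game's light level.
; On BeginPlay it runs the parent logic and caches the BigLeafGameMode.
; Each tick it interpolates between its minimum and maximum strength using the game mode's LightLevel and truncates the result to an integer Strength.
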(event `self.ReceiveBeginPlay`
  (`parent.ReceiveBeginPlay`)
  (bind _asbig_leaf_game_mode (cast `/Game/Blueprints/GameMode/BigLeafGameMode` (`GameplayStatics.GetGameMode`)))
  (set `self.BigLeafGameMode` _asbig_leaf_game_mode))

(event `self.ReceiveTick`
  (params (DeltaSeconds :type "Float (single-precision)"))
  (set `self.Strength` (`KismetMathLibrary.FTrunc` (`KismetMathLibrary.Lerp` (`KismetMathLibrary.Conv_IntToDouble` (`self.MinStrength`)) (`KismetMathLibrary.Conv_IntToDouble` (`self.MaxStrength`)) (`/Game/Blueprints/GameMode/BigLeafGameMode.LightLevel` (`self.BigLeafGameMode`))))))

(fn `UserConstructionScript`
  (`parent.UserConstructionScript`))