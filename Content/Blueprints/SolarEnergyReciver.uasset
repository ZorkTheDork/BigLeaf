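; Solar energy receiver that tracks how much solar energy reaches it from the energy zones registered with it.
; Zones are held in a set, and adding or removing one, or a refresh event bound through the Fox game mode, recalculates the level.
; The recalculation adds sun zones and subtracts shade zones, clamping after each step to the 0–255 range, then signals that the resource changed.
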(event `self.ReceiveBeginPlay`
  (bind _asfox_game_mode (`/Game/Blueprints/ActorComponentMacros.GetFoxGameMode`))
  (add `/Game/Blueprints/GameMode/BigLeafGameMode.RefreshResourceReceivers` _asfox_game_mode (delegate `Event RefreshResourceRecieivers`)))

(event `Event RefreshResourceRecieivers`
  (`self.RefreshIncomingEnergyLevel`))

(fn `AddSolarEnergyZone`
  (params (EnergyZone :type "/Game/Blueprints/SolarEnergyZone Object Reference"))
  (`BlueprintSetLibrary.Set_Add` (`self.EnergyZones`) EnergyZone)
  (`self.RefreshIncomingEnergyLevel`))

(fn `GetCurrentEnergyLevel`
  (returns (EnergyLevel :type Integer))
  (return (`self.EnergyLevelReceiving`)))

(fn `RefreshIncomingEnergyLevel`
  (locals (totalEnergyOfZones :type Integer))
  (set `local.totalEnergyOfZones` 0)
  (bind _result (`BlueprintSetLibrary.Set_ToArray` (`self.EnergyZones`)))
  (for _array_element _result
    (if (`/Game/Blueprints/SolarEnergyZone.IsShade` _array_element)
      ;[1 1 1] IsShade and reduces energy
      (set `local.totalEnergyOfZones` (`KismetMathLibrary.Max` (- (`local.totalEnergyOfZones`) (`/Game/Blueprints/SolarEnergyZone.Strength` _array_element))))
      (else
        ;[1 1 1] Is not shade and adds energy
        (set `local.totalEnergyOfZones` (`KismetMathLibrary.Min` (+ (`/Game/Blueprints/SolarEnergyZone.Strength` _array_element) (`local.totalEnergyOfZones`)) 255)))))
  (set `self.EnergyLevelReceiving` (`local.totalEnergyOfZones`))
  (`self.ResourceChanged`)
  (return))

(fn `RemoveSolarEnergyZone`
  (params (EnergyZone :type "/Game/Blueprints/SolarEnergyZone Object Reference"))
  (`BlueprintSetLibrary.Set_Remove` (`self.EnergyZones`) EnergyZone)
  (`self.RefreshIncomingEnergyLevel`))