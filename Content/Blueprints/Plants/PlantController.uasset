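; Plant controller component that simulates growth, decay, death and harvesting for its owning plant actor.
; Hydration and sunlight receivers are graded against ranges and combined into a Bad, Okay or Good state, refreshed on resource changes and game-mode simulation ticks.
; Good ticks add growth and heal decay, Okay holds steady, and Bad decays toward death after a grace period.
; Harvesting mature plants spawns an actor, then destroys or shrinks the plant.
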(event `self.ReceiveBeginPlay`
  (bind _returnvalue (`self.GetOwner`))
  (bind _asfox_game_mode (`/Game/Blueprints/ActorComponentMacros.GetFoxGameMode`))
  (add `/Game/Blueprints/GameMode/BigLeafGameMode.SimulatePlants` _asfox_game_mode (delegate `Event SimulatePlants`))
  (set `self.HydrationReceiver` (`Actor.GetComponentByClass` _returnvalue "/Game/Blueprints/HydrationReceiver.HydrationReceiver_C"))
  (set `self.SolarEnergyReciever` (`Actor.GetComponentByClass` _returnvalue "/Game/Blueprints/SolarEnergyReciver.SolarEnergyReciver_C"))
  (`self.BindOnResourceChanged`))

(event `Event SimulatePlants`
  (`self.UpdateResourceStates`)
  (`self.PlantSimulationTick`))

(event `BindOnResourceChanged`
  (add `/Game/Blueprints/HydrationReceiver.ResourceChanged` (`self.HydrationReceiver`) (delegate `UpdateResourceStates`))
  (add `/Game/Blueprints/SolarEnergyReciver.ResourceChanged` (`self.SolarEnergyReciever`) (delegate `UpdateResourceStates`)))

(event `UpdateResourceStates`
  (`self.UpdateHydrationState`)
  (`self.UpdateSunlightState`)
  (`self.UpdateOverallResourceState`))

(event `UpdateHydrationState`
  (set `self.HydrationState` (`/Game/Blueprints/ActorComponentMacros.PlantResourceStateFromRangeSelect` (`/Game/Blueprints/HydrationReceiver.HydrationLevelReceiving` (`self.HydrationReceiver`)) (`self.MaxHydrationForGrowth`) (`self.MinHydrationForGrowth`))))

(event `UpdateSunlightState`
  (set `self.SunliightState` (`/Game/Blueprints/ActorComponentMacros.PlantResourceStateFromRangeSelect` (`/Game/Blueprints/SolarEnergyReciver.EnergyLevelReceiving` (`self.SolarEnergyReciever`)) (`self.MaxSolarEnergyForGrowth`) (`self.MinSolarEnergyForGrowth`))))

(event `UpdateOverallResourceState`
  (bind _sunliightstate (`self.SunliightState`))
  (switch `/Game/Blueprints/LowGoodHighEnum` (`self.HydrationState`)
    (:`NewEnumerator0`
      (switch `/Game/Blueprints/LowGoodHighEnum` _sunliightstate
        (:`NewEnumerator0`
          (set `self.PlantOverallResourceState` "NewEnumerator0" :!label _label))
        (:`NewEnumerator1`
          (set `self.PlantOverallResourceState` "NewEnumerator1" :!label _label_2))
        (:`NewEnumerator2`
          (goto _label))))
    (:`NewEnumerator1`
      (switch `/Game/Blueprints/LowGoodHighEnum` _sunliightstate
        (:`NewEnumerator0`
          (goto _label_2))
        (:`NewEnumerator1`
          (set `self.PlantOverallResourceState` "NewEnumerator2"))
        (:`NewEnumerator2`
          (goto _label_2))))
    (:`NewEnumerator2`
      (switch `/Game/Blueprints/LowGoodHighEnum` _sunliightstate
        (:`NewEnumerator0`
          (goto _label))
        (:`NewEnumerator1`
          (goto _label_2))
        (:`NewEnumerator2`
          (goto _label))))))

(event `PlantSimulationTick`
  ;[1 1 1] Plant simulation
  (if (not (`self.IsDead`))
    (switch `/Game/Blueprints/GoodOkayBadEnum` (`self.PlantOverallResourceState`)
      (:`NewEnumerator0`
        (bind _result (`/Engine/EditorBlueprintResources/StandardMacros.IncrementInt` (`self.CurrentNonGrowthTicks`))
          (:`  `
            (if (>= _result (`self.NonGrowthTicksUntilDecay`))
              (`self.DecayTick`)))))
      (:`NewEnumerator2`
        (set `self.CurrentNonGrowthTicks` 0)
        (`self.GrowthTick`)))))

(event `GrowthTick`
  ;[1 1 1] Plant simulation
  (set `self.VegitativeGrowthPoints` (`KismetMathLibrary.Min` (+ (`self.GrowthPerGrowTick`) (`self.VegitativeGrowthPoints`)) (`self.MaxGrowthSize`)))
  (set `self.DecayPoints` (`KismetMathLibrary.Max` (- (`self.DecayPoints`) (`self.DecayRecoverPerGrowthTick`)))))

(event `DecayTick`
  ;[1 1 1] Plant simulation
  (bind _output_get (set `self.DecayPoints` (`KismetMathLibrary.Min` (+ (`self.DecayPoints`) (`self.DecayPerDecayTick`)) (`self.MaxDecayAmount`))))
  (if (>= _output_get (`self.MaxDecayAmount`))
    (set `self.IsDead` true)))

(event `BindOnHarvest`
  (add `self.OnHarvest` (delegate `OnHarvestHandler`)))

(event `OnHarvestHandler`
  (if (and (`self.IsHarvestable`) (>= (`self.VegitativeGrowthPoints`) (`self.GrowthSizeHarvestableAt`)))
    (`|SpawnActorFromClass` (`self.ActorToSpawnOnHarvest`) (`Actor.GetTransform` (`self.GetOwner`)) "AdjustIfPossibleButAlwaysSpawn" "OverrideRootScale" null null)
    (if (`self.IsHarvestingDestroy`)
      (`Actor.K2_DestroyActor` (`self.GetOwner`))
      (else
        (set `self.VegitativeGrowthPoints` (`self.GrowthSizeAfterHarvest`))))))