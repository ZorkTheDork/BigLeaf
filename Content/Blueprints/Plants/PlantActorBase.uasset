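; Base plant actor that visually reflects the growth, decay and health held by its PlantController.
; Each Tick steps through LifeStages as growth points cross thresholds, dropping back when growth regresses, such as after harvest.
; The current stage sets the mesh, with scale interpolated by growth progress.
; New dynamic material instances every Tick tint the mesh toward DeadColor with decay and color HealthSphere by resource state.
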(event `self.ReceiveBeginPlay`
  (set `self.CurrentLifeStage` (`self.StartingLifeStage`))
  (set `self.FinalLifeStage` (- (`KismetArrayLibrary.Array_Length` (`self.LifeStages`)) 1))
  (`self.UpdateLifeStageState`))

(event `self.ReceiveTick`
  (params (DeltaSeconds :type "Float (single-precision)"))
  (`self.UpdateaHealthSphere`)
  (`self.UpdateLifeStage`)
  (`self.UpdateMesh`)
  (`self.UpdateMaterial`)
  (`self.UpdateSize`))

(event `UpdateSize`
  (bind (_stagename _growththreshold _stagemesh _startingscale _endscale) (break `/Game/Blueprints/Plants/PlantLifeStage` (`|GetArrayItem` (`self.LifeStages`) (`self.CurrentLifeStage`))))
  (bind (_stagename_2 _growththreshold_2) (break `/Game/Blueprints/Plants/PlantLifeStage` (`|GetArrayItem` (`self.LifeStages`) (`self.CurrentLifeStage`))))
  (`SceneComponent.SetWorldScale3D` (`self.MainMesh`) (* (1.0 1.0 1.0) (`KismetMathLibrary.Lerp` _startingscale _endscale (/ (`KismetMathLibrary.Conv_IntToDouble` (- (`/Game/Blueprints/Plants/PlantController.VegitativeGrowthPoints` (`self.PlantController`)) _growththreshold_2)) (`KismetMathLibrary.Conv_IntToDouble` (- (`self.NextGrowthThreshold`) _growththreshold_2)))))))

(event `UpdateMesh`
  (`StaticMeshComponent.SetStaticMesh` (`self.MainMesh`) (`.StageMesh_15_79EEEC844035F3C2BE172B8B1B3944B4` (break `/Game/Blueprints/Plants/PlantLifeStage` (`|GetArrayItem` (`self.LifeStages`) (`self.CurrentLifeStage`))))) ; TEMP Set mesh to FullyGrownMesh
)

(event `UpdateMaterial`
  (bind _mainmesh (`self.MainMesh`))
  (bind _plantcontroller (`self.PlantController`))
  (bind _returnvalue (`PrimitiveComponent.CreateDynamicMaterialInstance` _mainmesh 0 (`PrimitiveComponent.GetMaterial` _mainmesh 0) "None"))
  (`MaterialInstanceDynamic.SetVectorParameterValue` _returnvalue "OverrideColor" (`self.DeadColor`))
  (`MaterialInstanceDynamic.SetScalarParameterValue` _returnvalue "OverrideColorStrength" (/ (`KismetMathLibrary.Conv_IntToDouble` (`/Game/Blueprints/Plants/PlantController.DecayPoints` _plantcontroller)) (`KismetMathLibrary.Conv_IntToDouble` (`/Game/Blueprints/Plants/PlantController.MaxDecayAmount` _plantcontroller)))))

(event `UpdateaHealthSphere`
  (bind _healthsphere (`self.HealthSphere`))
  (bind _returnvalue (`PrimitiveComponent.CreateDynamicMaterialInstance` _healthsphere 0 (`PrimitiveComponent.GetMaterial` _healthsphere 0) "None"))
  (`MaterialInstanceDynamic.SetVectorParameterValue` _returnvalue "Color" (select `/Game/Blueprints/GoodOkayBadEnum` (`/Game/Blueprints/Plants/PlantController.PlantOverallResourceState` (`self.PlantController`)) :`NewEnumerator0` (struct :`R` 1.0 :`G` 0.008761 :`A` 1.0) :`NewEnumerator1` (struct :`R` 1.0 :`G` 0.88273 :`A` 1.0) :`NewEnumerator2` (struct :`R` 0.11497 :`G` 1.0 :`A` 1.0) :!type "LinearColor Structure")) ; Set color based on plant overall health state
)

(event `UpdateLifeStage`
  (if (and (>= (- (`self.CurrentLifeStage`) 1) 0) (< (`/Game/Blueprints/Plants/PlantController.VegitativeGrowthPoints` (`self.PlantController`)) (`.GrowthThreshold_8_D70A0E644C7EC69CA1234A957100B97B` (break `/Game/Blueprints/Plants/PlantLifeStage` (`|GetArrayItem` (`self.LifeStages`) (`self.CurrentLifeStage`))))))
    (`/Engine/EditorBlueprintResources/StandardMacros.DecrementInt` (`self.CurrentLifeStage`)
      (:`  `
        (if (> (`/Game/Blueprints/Plants/PlantController.VegitativeGrowthPoints` (`self.PlantController`)) (`self.NextGrowthThreshold`))
          (if (< (`self.CurrentLifeStage`) (`self.FinalLifeStage`))
            (`/Engine/EditorBlueprintResources/StandardMacros.IncrementInt` (`self.CurrentLifeStage`)
              (:`  `
                (`self.UpdateLifeStageState`)))))))))

(event `UpdateLifeStageState`
  (set `self.CurrentLifeStageName` (`.StageName_4_084396F44E584D5D848369B2D0E6F353` (break `/Game/Blueprints/Plants/PlantLifeStage` (`|GetArrayItem` (`self.LifeStages`) (`self.CurrentLifeStage`)))))
  (if (>= (`self.FinalLifeStage`) (+ (`self.CurrentLifeStage`) 1))
    (set `self.NextGrowthThreshold` (`.GrowthThreshold_8_D70A0E644C7EC69CA1234A957100B97B` (break `/Game/Blueprints/Plants/PlantLifeStage` (`|GetArrayItem` (`self.LifeStages`) (+ (`self.CurrentLifeStage`) 1)))))
    (else
      (set `self.NextGrowthThreshold` (`/Game/Blueprints/Plants/PlantController.MaxGrowthSize` (`self.PlantController`))))))

(fn `UserConstructionScript`)