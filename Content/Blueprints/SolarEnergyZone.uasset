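; Solar energy zone volume that registers itself with the SolarEnergyReciver component of actors inside it.
; On BeginPlay, OnReset and ReInit (also called from the construction script), it scans ZoneTriggerCollider for overlapping PlantActorBase actors and adds itself to their receivers.
; Begin and end overlap events add or remove the zone for any actor with that component, without the plant class filter.
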(event `self.ReceiveBeginPlay`
  (bind _zonetriggercollider (`self.ZoneTriggerCollider`))
  (bind _outactors (`KismetSystemLibrary.ComponentOverlapActors` _zonetriggercollider (`SceneComponent.K2_GetComponentToWorld` _zonetriggercollider) (`|MakeArray` "ObjectTypeQuery1" "ObjectTypeQuery2" :!type "EObjectTypeQuery Enum") "/Game/Blueprints/Plants/PlantActorBase.PlantActorBase_C" :!label _label))
  (for _array_element _outactors
    (bind _returnvalue (`self.GetComponentByClass` _array_element "/Game/Blueprints/SolarEnergyReciver.SolarEnergyReciver_C"))
    (if (!= _returnvalue null)
      (`/Game/Blueprints/SolarEnergyReciver.AddSolarEnergyZone` _returnvalue self))))

(event `self.K2_OnReset`
  (goto _label))

(event `ReInit`
  (goto _label))

(event `self.ReceiveActorBeginOverlap`
  (params (OtherActor :type "Actor Object Reference"))
  (bind _returnvalue (`self.GetComponentByClass` OtherActor "/Game/Blueprints/SolarEnergyReciver.SolarEnergyReciver_C"))
  (if (!= _returnvalue null)
    (`/Game/Blueprints/SolarEnergyReciver.AddSolarEnergyZone` _returnvalue self)))

(event `self.ReceiveActorEndOverlap`
  (params (OtherActor :type "Actor Object Reference"))
  (bind _returnvalue (`self.GetComponentByClass` OtherActor "/Game/Blueprints/SolarEnergyReciver.SolarEnergyReciver_C"))
  (if (!= _returnvalue null)
    (`/Game/Blueprints/SolarEnergyReciver.RemoveSolarEnergyZone` _returnvalue self)))

(fn `UserConstructionScript`
  (`self.ReInit`))