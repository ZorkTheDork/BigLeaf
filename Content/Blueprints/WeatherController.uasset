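; Weather controller that plays a one-shot timed storm: clouds and gloom shift, rain runs for a while, then conditions ease.
; BeginPlay attaches the rain particle's owning actor to the player and drives the timeline with delays, setting target values and toggling the particles.
; Tick steps sky cloud opacity and the MP_Global Gloom and RainLevel parameters toward those targets at ChangeRate-scaled speeds, refreshing the sky material every frame.
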(event `self.ReceiveBeginPlay`
  (`KismetSystemLibrary.Delay` 0.2)
  (`self.K2_AttachToComponent` (`ActorComponent.GetOwner` (`self.PS_Rain`)) (`Actor.RootComponent` (`GameplayStatics.GetPlayerCharacter` 0)) "None" "SnapToTarget" "SnapToTarget" "SnapToTarget" true)
  (`self.K2_AddActorLocalOffset` (-100.0 -20.0 0.0))
  (`KismetSystemLibrary.Delay` 5.0)
  (set `self.TargetCloudOpacity` 20.0)
  (set `self.GloomLevel` 1e-06)
  (`KismetSystemLibrary.Delay` 40.0)
  (`self.ToggleRain` true)
  (`KismetSystemLibrary.Delay` 45.0)
  (`self.ToggleRain` false)
  (set `self.TargetCloudOpacity` 0.7)
  (set `self.GloomLevel` 1.0))

(event `self.ReceiveTick`
  (params (DeltaSeconds :type "Float (single-precision)"))
  (bind _cloud_opacity (`/Engine/EngineSky/BP_Sky_Sphere.Cloud opacity` (`self.Sky`)))
  (bind _returnvalue (- (`self.TargetCloudOpacity`) _cloud_opacity))
  (bind _returnvalue_2 (`KismetMaterialLibrary.GetScalarParameterValue` "/Game/Materials/MP_Global.MP_Global" "Gloom"))
  (bind _returnvalue_3 (- (`self.GloomLevel`) _returnvalue_2))
  (if (> (`KismetMathLibrary.Abs` _returnvalue_3) 0.1)
    (`KismetMaterialLibrary.SetScalarParameterValue` "/Game/Materials/MP_Global.MP_Global" "Gloom" (+ _returnvalue_2 (* (* (`self.ChangeRate`) (`KismetMathLibrary.SelectFloat` 1.0 -1.0 (> _returnvalue_3 0.0))) 0.25))))
  (if (> (`KismetMathLibrary.Abs` _returnvalue) 0.1)
    (set `/Engine/EngineSky/BP_Sky_Sphere.Cloud opacity` (+ _cloud_opacity (* (* (`self.ChangeRate`) (`KismetMathLibrary.SelectFloat` 1.0 -1.0 (> _returnvalue 0.0))) 4.0)) (`self.Sky`)))
  (bind _returnvalue_4 (`KismetMaterialLibrary.GetScalarParameterValue` "/Game/Materials/MP_Global.MP_Global" "RainLevel"))
  (bind _returnvalue_5 (- (`self.RainLevel`) _returnvalue_4))
  (if (> (`KismetMathLibrary.Abs` _returnvalue_5) 0.1)
    (`KismetMaterialLibrary.SetScalarParameterValue` "/Game/Materials/MP_Global.MP_Global" "RainLevel" (+ _returnvalue_4 (* (`self.ChangeRate`) (`KismetMathLibrary.SelectFloat` 1.0 -1.0 (> _returnvalue_5 0.0))))))
  (`/Engine/EngineSky/BP_Sky_Sphere.RefreshMaterial` (`self.Sky`))
  (if (>= (`KismetMathLibrary.RandomIntegerInRange` 0 5) 4)
    _))

(event `ToggleRain`
  (params (Enable :type Boolean))
  (if Enable
    (`ActorComponent.SetActive` (`self.PS_Rain`) true false)
    (set `self.RainLevel` 0.8)
    (else
      (`ActorComponent.SetActive` (`self.PS_Rain`) false false)
      (set `self.RainLevel` 0.1))))

(fn `UserConstructionScript`)