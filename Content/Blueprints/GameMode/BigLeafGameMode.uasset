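; Game mode for BigLeaf that plays a 2D sound at start and drives the plant simulation.
; Each tick it caches LightLevel from the MP_Global material parameter collection, then periodically calls resource-receiver refresh and plant simulation at PlantSimulationTickRate.
; OncePerXSeconds times this using game time modulo the period within a tolerance, with a DoOnce that resets at the half-period to prevent repeat firing.
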(event `self.ReceiveBeginPlay`
  (`GameplayStatics.PlaySound2D` null 1.0 1.0 0.0 null null))

(event `self.ReceiveTick`
  (params (DeltaSeconds :type "Float (single-precision)"))
  (bind _returnvalue (`KismetMaterialLibrary.GetScalarParameterValue` "/Game/Materials/MP_Global.MP_Global" "LightLevel"))
  (set `self.LightLevel` _returnvalue)
  (`self.OncePerXSeconds` (`self.PlantSimulationTickRate`)
    (:`true`
      (`self.RefreshResourceReceivers`)
      (`self.SimulatePlants`))))

(fn `UserConstructionScript`)