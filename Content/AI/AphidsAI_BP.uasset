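; AI controller for aphids that runs the AphidsAI_BT behavior tree and picks a plant to eat.
; On each perception update it scans all Plant actors in the level, not the perceived ones, and writes the first tagged one whose CanEatMessage returns true to the blackboard target key.
; The tag check tests each plant against its own first tag, and the CanSeePlant sight logic is disconnected.
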(event `self.ReceiveBeginPlay`
  (`self.RunBehaviorTree` "/Game/AI/AphidsAI_BT.AphidsAI_BT"))

(event `self.AIPerception.OnPerceptionUpdated`
  (params (UpdatedActors :type "Array of Actor Object Reference (by ref)"))
  ;[1 1 1] Go to Plant
  (bind _outactors (`GameplayStatics.GetAllActorsOfClass` "/Game/Blueprints/Plant.Plant_C"))
  (for _array_element _outactors
    (if (`self.ActorHasTag` _array_element (`|GetArrayItem` (`Actor.Tags` _array_element)))
      (bind _caneat_ (message `/Game/Blueprints/canEatPlant.CanEat?` _array_element null))
      (if _caneat_
        (`BlackboardComponent.SetValueAsObject` (`AIBlueprintHelperLibrary.GetBlackboard` null) (`self.TargetActorKeyName`) _array_element)
        (break)))))

(event `self.AIPerception.OnTargetPerceptionUpdated`
  (params (Actor :type "Actor Object Reference") (Stimulus :type "AIStimulus Structure")))

(fn `UserConstructionScript`)