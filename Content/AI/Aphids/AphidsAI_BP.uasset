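; AI controller for aphids that sends them toward plants they can eat.
; On begin play it runs the AphidsAI_BT behavior tree.
; When perception updates, it writes the first perceived actor that implements CanEatPlant and answers true to CanEatMessage into the blackboard's target actor key.
; A disconnected GetAllActorsOfClass lookup for plants remains as an unused alternative.
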(event `self.ReceiveBeginPlay`
  (`self.RunBehaviorTree` "/Game/AI/Aphids/AphidsAI_BT.AphidsAI_BT"))

(event `self.AIPerception.OnPerceptionUpdated`
  (params (UpdatedActors :type "Array of Actor Object Reference (by ref)"))
  ;[1 1 1] Go to Plant
  (for _array_element UpdatedActors
    (if (`KismetSystemLibrary.DoesImplementInterface` _array_element "/Game/Blueprints/canEatPlant.canEatPlant_C")
      (bind _caneat_ (message `/Game/Blueprints/canEatPlant.CanEat?` _array_element null))
      (if _caneat_
        (`BlackboardComponent.SetValueAsObject` (`AIBlueprintHelperLibrary.GetBlackboard` null) (`self.TargetActorKeyName`) _array_element)
        (break)))))

(fn `UserConstructionScript`)